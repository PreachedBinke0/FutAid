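; Crowd manager that bakes placed BP_Crowd_VAT actors into instanced meshes for a stadium crowd.
; The HornearEstadio event clears three HISMs (base, blue, red), then adds an instance at each actor's transform to the one matching its color index.
; Per-instance custom data carries the selected animation's start and end frames, a random value and a constant for vertex animation.
; Baked source actors are hidden in game.
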(event Custom|HornearEstadio
  (Components|InstancedStaticMesh|ClearInstances (Variables|Default|GetHISM_Base))
  (Components|InstancedStaticMesh|ClearInstances (Variables|Default|GetHISM_Blue))
  (Components|InstancedStaticMesh|ClearInstances (Variables|Default|GetHISM_Red))
  (bind _outactors (Actor|GetAllActorsOfClass "/Game/Assets/Crowd/BP_Crowd_VAT.BP_Crowd_VAT_C"))
  (for _array_element _outactors
    (switch int (Variables|/Game/Assets/Crowd/BP_Crowd_VAT.BP_Crowd_VAT_C|GetCurrentColorIndex _array_element)
      (:0
        (bind _returnvalue (Components|InstancedStaticMesh|AddInstance (Variables|Default|GetHISM_Blue) (Transformation|GetActorTransform _array_element) true))
        (Components|InstancedStaticMesh|SetCustomDataValue (Variables|Default|GetHISM_Blue) _returnvalue 2 (Math|Conversions|ToFloat(Integer) (Utilities|Array|Get(acopy) (Variables|/Game/Assets/Crowd/BP_Crowd_VAT.BP_Crowd_VAT_C|GetAnimationStartFrames _array_element) (Variables|/Game/Assets/Crowd/BP_Crowd_VAT.BP_Crowd_VAT_C|GetCurrentAnimIndex _array_element))) false)
        (Components|InstancedStaticMesh|SetCustomDataValue (Variables|Default|GetHISM_Blue) _returnvalue 3 (Math|Conversions|ToFloat(Integer) (Utilities|Array|Get(acopy) (Variables|/Game/Assets/Crowd/BP_Crowd_VAT.BP_Crowd_VAT_C|GetAnimationEndFrames _array_element) (Variables|/Game/Assets/Crowd/BP_Crowd_VAT.BP_Crowd_VAT_C|GetCurrentAnimIndex _array_element))) false)
        (Components|InstancedStaticMesh|SetCustomDataValue (Variables|Default|GetHISM_Blue) _returnvalue 1 1.0 false)
        (Components|InstancedStaticMesh|SetCustomDataValue (Variables|Default|GetHISM_Blue) _returnvalue 0 (Math|Random|RandomFloatinRange 0.0 3.0) false)
        (Rendering|SetActorHiddenInGame _array_element true))
      (:1
        (bind _returnvalue_2 (Components|InstancedStaticMesh|AddInstance (Variables|Default|GetHISM_Base) (Transformation|GetActorTransform _array_element) true))
        (Components|InstancedStaticMesh|SetCustomDataValue (Variables|Default|GetHISM_Base) _returnvalue_2 2 (Math|Conversions|ToFloat(Integer) (Utilities|Array|Get(acopy) (Variables|/Game/Assets/Crowd/BP_Crowd_VAT.BP_Crowd_VAT_C|GetAnimationStartFrames _array_element) (Variables|/Game/Assets/Crowd/BP_Crowd_VAT.BP_Crowd_VAT_C|GetCurrentAnimIndex _array_element))) false)
        (Components|InstancedStaticMesh|SetCustomDataValue (Variables|Default|GetHISM_Base) _returnvalue_2 3 (Math|Conversions|ToFloat(Integer) (Utilities|Array|Get(acopy) (Variables|/Game/Assets/Crowd/BP_Crowd_VAT.BP_Crowd_VAT_C|GetAnimationEndFrames _array_element) (Variables|/Game/Assets/Crowd/BP_Crowd_VAT.BP_Crowd_VAT_C|GetCurrentAnimIndex _array_element))) false)
        (Components|InstancedStaticMesh|SetCustomDataValue (Variables|Default|GetHISM_Base) _returnvalue_2 1 1.0 false)
        (Components|InstancedStaticMesh|SetCustomDataValue (Variables|Default|GetHISM_Base) _returnvalue_2 0 (Math|Random|RandomFloatinRange 0.0 3.0) false)
        (Rendering|SetActorHiddenInGame _array_element true))
      (:2
        (bind _returnvalue_3 (Components|InstancedStaticMesh|AddInstance (Variables|Default|GetHISM_Red) (Transformation|GetActorTransform _array_element) true))
        (Components|InstancedStaticMesh|SetCustomDataValue (Variables|Default|GetHISM_Red) _returnvalue_3 2 (Math|Conversions|ToFloat(Integer) (Utilities|Array|Get(acopy) (Variables|/Game/Assets/Crowd/BP_Crowd_VAT.BP_Crowd_VAT_C|GetAnimationStartFrames _array_element) (Variables|/Game/Assets/Crowd/BP_Crowd_VAT.BP_Crowd_VAT_C|GetCurrentAnimIndex _array_element))) false)
        (Components|InstancedStaticMesh|SetCustomDataValue (Variables|Default|GetHISM_Red) _returnvalue_3 3 (Math|Conversions|ToFloat(Integer) (Utilities|Array|Get(acopy) (Variables|/Game/Assets/Crowd/BP_Crowd_VAT.BP_Crowd_VAT_C|GetAnimationEndFrames _array_element) (Variables|/Game/Assets/Crowd/BP_Crowd_VAT.BP_Crowd_VAT_C|GetCurrentAnimIndex _array_element))) false)
        (Components|InstancedStaticMesh|SetCustomDataValue (Variables|Default|GetHISM_Red) _returnvalue_3 1 1.0 false)
        (Components|InstancedStaticMesh|SetCustomDataValue (Variables|Default|GetHISM_Red) _returnvalue_3 0 (Math|Random|RandomFloatinRange 0.0 3.0) false)
        (Rendering|SetActorHiddenInGame _array_element true)))))

(event EventBeginPlay)

(event Collision|EventActorBeginOverlap
  (params (OtherActor :type Actor%20Object%20Reference)))

(event EventTick
  (params (DeltaSeconds :type Float%20%28single-precision%29)))

(fn ConstructionScript)