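; BP_Crowd_VAT is a crowd character whose static mesh is animated through vertex animation texture materials.
; ActualizarVisuales, also run by the construction script, creates dynamic body and hair materials, picking one of three body color variants.
; It sets their StartFrame and EndFrame layer parameters from per-animation frame arrays to select the clip.
; GenerarPersonajeAleatoreo randomizes color and animation, then refreshes; the seated-dependent selection is left unconnected.
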(event Custom|Generar%20Personaje%20Aleatoreo
  (Variables|Default|SetCurrentColorIndex (Math|Random|RandomIntegerinRange 0 2))
  (Variables|Default|SetCurrentAnimIndex (Math|Random|RandomIntegerinRange 0 5))
  (CallFunction|ActualizarVisuales))

(event EventBeginPlay)

(event Collision|EventActorBeginOverlap
  (params (OtherActor :type Actor%20Object%20Reference)))

(event EventTick
  (params (DeltaSeconds :type Float%20%28single-precision%29)))

(fn ConstructionScript
  (CallFunction|ActualizarVisuales))

(fn ActualizarVisuales
  (bind _returnvalue (Rendering|Material|CreateDynamicMaterialInstance (Variables|Default|GetStaticMesh) 0 (Utilities|Select :Index (Variables|Default|GetCurrentColorIndex) :Option%200 "/Game/Assets/Crowd/Materials/MI_Body_Crowd_VAT.MI_Body_Crowd_VAT" :Option%201 "/Game/Assets/Crowd/Materials/MI_Body_Blue_Crowd_VAT.MI_Body_Blue_Crowd_VAT" :Option%202 "/Game/Assets/Crowd/Materials/MI_Body_Red_Crowd_VAT.MI_Body_Red_Crowd_VAT") "None" :!class /Script/Engine.PrimitiveComponent))
  (Rendering|Material|SetScalarParameterValuebyInfo _returnvalue (Utilities|Struct|MakeMaterialParameterInfo "StartFrame" "LayerParameter" 0) (Math|Conversions|ToFloat(Integer) (Utilities|Array|Get(acopy) (Variables|Default|GetAnimationStartFrames) (Variables|Default|GetCurrentAnimIndex))))
  (Rendering|Material|SetScalarParameterValuebyInfo _returnvalue (Utilities|Struct|MakeMaterialParameterInfo "EndFrame" "LayerParameter" 0) (Math|Conversions|ToFloat(Integer) (Utilities|Array|Get(acopy) (Variables|Default|GetAnimationEndFrames) (Variables|Default|GetCurrentAnimIndex))))
  (Rendering|Material|SetMaterial (Variables|Default|GetStaticMesh) 0 _returnvalue)
  (bind _returnvalue_2 (Rendering|Material|CreateDynamicMaterialInstance (Variables|Default|GetStaticMesh) 1 "/Game/Assets/Crowd/Materials/MI_Hair_Crowd_VAT.MI_Hair_Crowd_VAT" "None" :!class /Script/Engine.PrimitiveComponent))
  (Rendering|Material|SetScalarParameterValuebyInfo _returnvalue_2 (Utilities|Struct|MakeMaterialParameterInfo "StartFrame" "LayerParameter" 0) (Math|Conversions|ToFloat(Integer) (Utilities|Array|Get(acopy) (Variables|Default|GetAnimationStartFrames) (Variables|Default|GetCurrentAnimIndex))))
  (Rendering|Material|SetScalarParameterValuebyInfo _returnvalue_2 (Utilities|Struct|MakeMaterialParameterInfo "EndFrame" "LayerParameter" 0) (Math|Conversions|ToFloat(Integer) (Utilities|Array|Get(acopy) (Variables|Default|GetAnimationEndFrames) (Variables|Default|GetCurrentAnimIndex))))
  (Rendering|Material|SetMaterial (Variables|Default|GetStaticMesh) 1 _returnvalue_2))